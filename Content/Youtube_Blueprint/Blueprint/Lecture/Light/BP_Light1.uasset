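; BP_Light1 is an interactable light actor that toggles its point light with the F key.
; Overlapping its box collision enables player 0's input and toggles a text render; leaving disables input after a half-second delay and toggles the text again, with no check on which actor overlaps.
; The construction script hides the text and light initially and sets the light color from a variable.
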(event OnComponentBeginOverlap(BoxCollision)
  (params (OverlappedComponent :type Primitive%20Component%20Object%20Reference) (OtherActor :type Actor%20Object%20Reference) (OtherComp :type Primitive%20Component%20Object%20Reference) (OtherBodyIndex :type Integer) (bFromSweep :type Boolean) (SweepResult :type Hit%20Result%20Structure%20%28by%20ref%29))
  ;[1 1 1] Initial Visibility
  (Input|EnableInput (Game|GetPlayerController 0))
  (Rendering|ToggleVisibility (Variables|Default|GetTextRender) false))

(event OnComponentEndOverlap(BoxCollision)
  (params (OverlappedComponent :type Primitive%20Component%20Object%20Reference) (OtherActor :type Actor%20Object%20Reference) (OtherComp :type Primitive%20Component%20Object%20Reference) (OtherBodyIndex :type Integer))
  ;[1 1 1] Initial Visibility
  (Utilities|FlowControl|Delay 0.5)
  (Input|DisableInput (Game|GetPlayerController 0))
  (Rendering|ToggleVisibility (Variables|Default|GetTextRender) false))

(event Input|KeyboardEvents|F
  (params (Key :type Key%20Structure :default "None"))
  ;[1 1 1] Initial Visibility
  (:Pressed
    (Rendering|ToggleVisibility (Variables|Default|GetPointLight) false)))

(fn ConstructionScript
  (Rendering|SetVisibility (Variables|Default|GetTextRender) false false)
  (Rendering|Components|Light|SetLightColor (Variables|Default|GetPointLight) (Variables|Default|GetNew%20Light%20Color) true))