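; BP_Door is an interactive door that the player opens and closes while near it.
; A box collision enables input when a BP_ThirdPersonCharacter overlaps it and disables it on exit.
; E uses a FlipFlop to snap the door between two rotations.
; Q uses another FlipFlop to play or reverse the DoorRotation timeline, which animates the door's yaw.
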(event OnComponentBeginOverlap(BoxCollision)
  (params (OverlappedComponent :type Primitive%20Component%20Object%20Reference) (OtherActor :type Actor%20Object%20Reference) (OtherComp :type Primitive%20Component%20Object%20Reference) (OtherBodyIndex :type Integer) (bFromSweep :type Boolean) (SweepResult :type Hit%20Result%20Structure%20%28by%20ref%29))
  ;[1 1 1] Collision Check and Enable Input
  (Utilities|Casting|CastToBP_ThirdPersonCharacter OtherActor)
  (Input|EnableInput (Game|GetPlayerController 0)))

(event OnComponentEndOverlap(BoxCollision)
  (params (OverlappedComponent :type Primitive%20Component%20Object%20Reference) (OtherActor :type Actor%20Object%20Reference) (OtherComp :type Primitive%20Component%20Object%20Reference) (OtherBodyIndex :type Integer))
  ;[1 1 1] Collision Check and Enable Input
  (Utilities|Casting|CastToBP_ThirdPersonCharacter OtherActor)
  (Input|DisableInput (Game|GetPlayerController 0)))

(event Input|KeyboardEvents|E
  (params (Key :type Key%20Structure :default "None"))
  (bind _door (Variables|Default|GetDoor))
  ;[1 1 1] Door Roation
  (:Pressed
    (Utilities|FlowControl|FlipFlop
      (:A
        (Transformation|SetRelativeRotation _door "0,90.000000, 0" false false))
      (:B
        (Transformation|SetRelativeRotation _door "0,0.000000, 0" false false)))))

(event Input|KeyboardEvents|Q
  (params (Key :type Key%20Structure :default "None"))
  ;[1 1 1] Timeline Animation Of Door
  (:Pressed
    (Utilities|FlowControl|FlipFlop
      (:A
        (bind _rotation_of_door (Timeline|Door%20Rotation Play)
          (:Update
            (Transformation|SetRelativeRotation (Variables|Default|GetDoor) (Math|Rotator|MakeRotator 0.0 0.0 _rotation_of_door) false false))))
      (:B
        (Timeline|Door%20Rotation Reverse)))))

(fn ConstructionScript)